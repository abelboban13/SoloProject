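; BP_Dummy is a target dummy character that takes hits and can be killed by a stealth back takedown.
; Damage plays a random hit montage, launches it along the player's facing and lowers health through BPCPlayerStats, ragdolling on death.
; StealthBackAssassin plays the victim montage, returns alignment location and rotation, and triggers a delayed ragdoll.
; Player overlap toggles the takedown prompt, which turns toward the camera with the health bar.
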(event OnComponentBeginOverlap(AssassinationRadius)
  (params (OverlappedComponent :type Primitive%20Component%20Object%20Reference) (OtherActor :type Actor%20Object%20Reference) (OtherComp :type Primitive%20Component%20Object%20Reference) (OtherBodyIndex :type Integer) (bFromSweep :type Boolean) (SweepResult :type Hit%20Result%20Structure%20%28by%20ref%29))
  (Utilities|Casting|CastToBP_ThirdPersonCharacter OtherActor)
  (Rendering|SetVisibility (Variables|Default|GetTakedown%20Widget) true false))

(event OnComponentEndOverlap(TakedownWidget)
  (params (OverlappedComponent :type Primitive%20Component%20Object%20Reference) (OtherActor :type Actor%20Object%20Reference) (OtherComp :type Primitive%20Component%20Object%20Reference) (OtherBodyIndex :type Integer))
  (Utilities|Casting|CastToBP_ThirdPersonCharacter OtherActor)
  (Rendering|SetVisibility (Variables|Default|GetTakedown%20Widget) false false))

(event Custom|Ragdoll
  (bind _bpc_playerstats (Variables|Default|GetBPC_PlayerStats))
  ;[1 1 1] Ragdoll
  (Default|DecreaseHealthDummy _bpc_playerstats (Variables|/Game/ThirdPerson/Blueprints/BPC_PlayerStats.BPC_PlayerStats_C|GetMax%20Health _bpc_playerstats))
  (Utilities|FlowControl|Sequence
    (:then_0
      (Utilities|FlowControl|Delay 2.5)
      (Physics|SetSimulatePhysics (Variables|Character|GetMesh) true)
      (Rendering|SetVisibility (Variables|Default|GetHealth%20Bar%20Widget) false false)
      (Components|DestroyComponent (Variables|Collision|GetCapsuleComponent)))
    (:then_1
      (Utilities|FlowControl|Delay 1.4)
      (Audio|PlaySoundatLocation "/Game/Audio/Grunts-Hits/MS_Death.MS_Death" (Transformation|GetActorLocation) "0, 0, 0" 1.0 1.0 0.0 0 0 0 0))))

(event Game|Damage|EventAnyDamage
  (params (Damage :type Float%20%28single-precision%29) (DamageType :type Damage%20Type%20Object%20Reference) (InstigatedBy :type Controller%20Object%20Reference) (DamageCauser :type Actor%20Object%20Reference))
  (bind _hitanims (Variables|Default|GetHitAnims))
  ;[1 1 1] Recieve Damage
  (Animation|PlayAnimMontage (Utilities|Array|Get(acopy) _hitanims (Math|Random|RandomIntegerinRange 0 (- (Utilities|Array|Length _hitanims) 1))) 1.0 "None")
  (bind _asbp_third_person_character (Utilities|Casting|CastToBP_ThirdPersonCharacter (Game|GetPlayerCharacter 0)))
  (Character|LaunchCharacter (* (Math|Vector|GetForwardVector (Transformation|GetActorRotation _asbp_third_person_character)) 5e+02) false false)
  (Audio|PlaySoundatLocation "/Game/Audio/Grunts-Hits/GetHitSFX.GetHitSFX" (Transformation|GetActorLocation) "0, 0, 0" 1.0 (Math|Random|RandomFloatinRange -1.5 0.5) 0.0 "/Game/Audio/SA_Character.SA_Character" 0 0 0)
  (bind _isplayerdead_ (Default|DecreaseHealthDummy (Variables|Default|GetBPC_PlayerStats) Damage))
  (if _isplayerdead_
    (Physics|SetSimulatePhysics (Variables|Character|GetMesh) true)
    (Audio|PlaySoundatLocation "/Game/Audio/Grunts-Hits/MS_Death.MS_Death" (Transformation|GetActorLocation) "0, 0, 0" 1.0 1.0 0.0 0 0 0 0)
    (Rendering|SetVisibility (Variables|Default|GetHealth%20Bar%20Widget) false false)
    (Components|DestroyComponent (Variables|Collision|GetCapsuleComponent))))

(event EventTick
  (params (DeltaSeconds :type Float%20%28single-precision%29))
  ;[1 1 1] Widget Rotation
  (Transformation|SetWorldRotation (Variables|Default|GetTakedown%20Widget) (Math|Rotator|FindLookatRotation (Transformation|GetWorldLocation (Variables|Default|GetTakedown%20Widget)) (Transformation|GetWorldLocation (Variables|/Script/Engine.PlayerCameraManager|GetTransformComponent (Game|GetPlayerCameraManager 0)))) false false))

(event EventBeginPlay
  (bind _aswb_dummy_health_bar (Utilities|Casting|CastToWB_DummyHealthBar (UserInterface|GetWidget (Variables|Default|GetHealth%20Bar%20Widget))))
  (Variables|Default|SetHealthBarUI _aswb_dummy_health_bar))

(fn ConstructionScript)

(fn StealthBackAssassin
  (bind _assassin_ref (Variables|Default|GetAssassin%20REF))
  (bind _returnvalue (Transformation|GetWorldLocation _assassin_ref))
  (Animation|PlayAnimMontage "/Game/Characters/PlayerCharacter/Animations/Assassinations/Paired_SneakNeckBreak_Vic_Montage.Paired_SneakNeckBreak_Vic_Montage" 1.0 "None")
  (CallFunction|Ragdoll)
  (Rendering|SetVisibility (Variables|Default|GetTakedown%20Widget) false false)
  (return (Math|Vector|MakeVector (.x _returnvalue) (.y _returnvalue) (.z _returnvalue)) (Transformation|GetActorRotation)))