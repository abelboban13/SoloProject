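; BP_Misc is an actor whose cube stretches vertically in response to the game mode's beat value.
; On BeginPlay it caches a reference to BP_ThirdPersonGameMode.
; Every tick it reads BeatValue and snaps the cube's relative Z scale between two heights at a threshold, leaving X and Y unchanged.
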(event EventBeginPlay
  (bind _asbp_third_person_game_mode (Utilities|Casting|CastToBP_ThirdPersonGameMode (Game|GetGameMode)))
  (Variables|Default|SetAs%20BP%20Third%20Person%20Game%20Mode _asbp_third_person_game_mode))

(event Collision|EventActorBeginOverlap
  (params (OtherActor :type Actor%20Object%20Reference)))

(event EventTick
  (params (DeltaSeconds :type Float%20%28single-precision%29))
  (bind _cube (Variables|Default|GetCube))
  (bind _relativescale3d (Variables|/Script/Engine.SceneComponent|GetRelativeScale3D _cube))
  (Transformation|SetRelativeScale3D _cube (Math|Vector|MakeVector (.x _relativescale3d) (.y _relativescale3d) (Math|Float|SelectFloat 2.0 1.0 (> (Variables|/Game/ThirdPerson/Blueprints/BP_ThirdPersonGameMode.BP_ThirdPersonGameMode_C|GetBeatValue (Variables|Default|GetAs%20BP%20Third%20Person%20Game%20Mode)) 0.5)))))

(fn ConstructionScript)