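; BP_Health is a pickup actor that restores the player's health on overlap.
; BeginPlay caches the player character, cast to BP_ThirdPersonCharacter.
; When that character overlaps the actor, its Health is set to a fixed 10 rather than incremented, and the pickup destroys itself.
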(event EventBeginPlay
  (bind _asbp_third_person_character (Utilities|Casting|CastToBP_ThirdPersonCharacter (Game|GetPlayerCharacter 0)))
  (Variables|Default|SetPlayerCharacter _asbp_third_person_character))

(event Collision|EventActorBeginOverlap
  (params (OtherActor :type Actor%20Object%20Reference))
  (if (== OtherActor (Variables|Default|GetPlayerCharacter))
    (Variables|/Game/ThirdPerson/Blueprints/BP_ThirdPersonCharacter.BP_ThirdPersonCharacter_C|SetHealth (Variables|Default|GetPlayerCharacter) 10)
    (Utilities|IsValid self
      (:Is%20Valid
        (Actor|DestroyActor)))))

(event EventTick
  (params (DeltaSeconds :type Float%20%28single-precision%29)))

(fn ConstructionScript)